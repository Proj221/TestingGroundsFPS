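; BP_InfiniteTerrain spawns a chain of terrain tiles and keeps a score.
; On BeginPlay it fills a NavMeshBoundsVolume pool, then runs a short, fixed loop that spawns a tile, waits, and calls NewTileCounquered to increment the score.
; SpawnTile hands each tile the shared pool and uses its attach point as the next spawn transform.
; GetScore exposes the count.
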(event EventBeginPlay
  (Class|InfiniteTerrain|PopulateBoundsVolumePool)
  (for _index (range 0 3)
    (CallFunction|SpawnTile)
    (Utilities|FlowControl|Delay 2.0)
    (CallFunction|NewTileCounquered)))

(fn ConstructionScript)

(fn SpawnTile
  (bind _returnvalue (Game|SpawnActorfromClass "/Game/Dynamic/a2_Terrain/Tile.Tile_C" (Variables|Default|GetNextTileTransform) "Undefined" 0 0))
  (Class|Tile|SetPool _returnvalue (Variables|Default|GetNavMeshBoundsVolumePool))
  (bind _attachpoint (Default|GetAttachPoint _returnvalue))
  (Variables|Default|SetNextTileTransform _attachpoint))

(fn NewTileCounquered
  (Math|Integer|IncrementInt (Variables|Default|GetMyScore)))

(fn GetScore
  (return (Variables|Default|GetMyScore)))