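; AI controller for NPCs that runs the GuardBehavior tree on the PatrolData blackboard.
; Perception updates set the enemy blackboard key to any sensed actor without the NPC tag and clear it when that actor is lost.
; Every tick it sets the controlled TP_Character to aim and shoot whenever the controller has a valid focus actor.
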(event OnTargetPerceptionUpdated(AIPerception)
  (params (Actor :type Actor%20Object%20Reference) (Stimulus :type AI%20Stimulus%20Structure))
  (bind _enemykey (Variables|Default|GetEnemyKey))
  (bind _blackboard_comp (Variables|Default|GetBlackboard%20Comp))
  (if (not (Actor|ActorHasTag Actor "NPC"))
    ;[1 1 1] Sense system
    (if (.bSuccessfullySensed (Utilities|Struct|BreakAIStimulus Stimulus))
      (AI|Components|Blackboard|SetValueasObject _blackboard_comp _enemykey Actor)
      (else
        (AI|Components|Blackboard|ClearValue _blackboard_comp _enemykey)))))

(event EventBeginPlay
  (bind _blackboardcomponent (Class|AIController|UseBlackboard "/Game/Dynamic/a1_NPC/AI/PatrolData.PatrolData"))
  (AI|RunBehaviorTree "/Game/Dynamic/a1_NPC/AI/GuardBehavior.GuardBehavior")
  (Variables|Default|SetBlackboard%20Comp _blackboardcomponent))

(event EventTick
  (params (DeltaSeconds :type Float%20%28single-precision%29))
  (bind _asue_4asp_character (Utilities|Casting|CastToTP_Character (Pawn|GetControlledPawn)))
  (bind _output_get (Variables|/Game/Dynamic/a1_NPC/Behavior/TP_Character.TP_Character_C|SetAiming _asue_4asp_character (Utilities|IsValid (Class|AIController|GetFocusActor))))
  (Variables|/Game/Dynamic/a1_NPC/Behavior/TP_Character.TP_Character_C|SetShooting _asue_4asp_character _output_get))

(fn ConstructionScript)